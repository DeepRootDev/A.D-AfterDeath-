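; MyCharacter_BP is a character Blueprint with a hold-to-charge projectile shot on the F key.
; Pressing F spawns a MyProjectile_BP at ProjectileLaunchPoint and plays a timeline that compounds its scale by 1% per update, so growth depends on frame rate.
; Releasing F stops the timeline, aligns the projectile to the launch point's rotation, sets its local forward velocity through ProjectileMovementComponent and clears the reference.
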(event Input|KeyboardEvents|F
  (params (Key :type Key%20Structure :default "None"))
  (:Pressed
    (bind _returnvalue (Game|SpawnActorfromClass "/Game/Blueprints/MyProjectile_BP.MyProjectile_BP_C" (Math|Transform|MakeTransform (Transformation|GetWorldLocation (Variables|Default|GetProjectileLaunchPoint))) "Undefined" 0 0))
    (Variables|Default|SetProjectile _returnvalue)
    (Timeline|ProjectileTimeline PlayFromStart
      (:Update
        (Transformation|SetActorScale3D (Variables|Default|GetProjectile) (* (Transformation|GetActorScale3D (Variables|Default|GetProjectile)) 1.01)))))
  (:Released
    (Utilities|FlowControl|Sequence
      (:then_0
        (Timeline|ProjectileTimeline Stop))
      (:then_1
        (Development|PrintString "Fire")
        (if (and (!= (Variables|Default|GetProjectile) 0) (!= (Actor|GetComponentbyClass (Variables|Default|GetProjectile) "/Script/Engine.ProjectileMovementComponent") 0))
          (Transformation|SetActorRotation (Variables|Default|GetProjectile) (Transformation|GetWorldRotation (Variables|Default|GetProjectileLaunchPoint)))
          (Game|Components|ProjectileMovement|SetVelocityinLocalSpace (Actor|GetComponentbyClass (Variables|Default|GetProjectile) "/Script/Engine.ProjectileMovementComponent") "1500.000000,0.000000, 0")
          (Variables|Default|SetProjectile 0))))))

(fn ConstructionScript)